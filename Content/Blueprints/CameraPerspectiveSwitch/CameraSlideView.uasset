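; CameraSlideView is a trigger-volume actor that switches the player's camera to a slide view while they are inside it.
; When BP_PlayerCharacter enters BoxCollision, it caches the player and swaps the active FollowCamera for SlideCamera.
; When any overlap ends, it restores FollowCamera on the cached player if SlideCamera is active, without checking which actor left.
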(event OnComponentBeginOverlap(BoxCollision)
  (params (OverlappedComponent :type Primitive%20Component%20Object%20Reference) (OtherActor :type Actor%20Object%20Reference) (OtherComp :type Primitive%20Component%20Object%20Reference) (OtherBodyIndex :type Integer) (bFromSweep :type Boolean) (SweepResult :type Hit%20Result%20Structure%20%28by%20ref%29))
  (bind _asbp_player_character (Utilities|Casting|CastToBP_PlayerCharacter OtherActor))
  (Variables|Default|SetPlayerRef _asbp_player_character)
  (if (Components|Activation|IsActive (Variables|/Game/Blueprints/AmyPlayerCharacter/CharacterBlueprints/BP_PlayerCharacter.BP_PlayerCharacter_C|GetFollowCamera (Variables|Default|GetPlayerRef)))
    (Components|Activation|SetActive (Variables|/Game/Blueprints/AmyPlayerCharacter/CharacterBlueprints/BP_PlayerCharacter.BP_PlayerCharacter_C|GetSlideCamera (Variables|Default|GetPlayerRef)) true false)
    (Components|Activation|SetActive (Variables|/Game/Blueprints/AmyPlayerCharacter/CharacterBlueprints/BP_PlayerCharacter.BP_PlayerCharacter_C|GetFollowCamera (Variables|Default|GetPlayerRef)) false false)))

(event OnComponentEndOverlap(BoxCollision)
  (params (OverlappedComponent :type Primitive%20Component%20Object%20Reference) (OtherActor :type Actor%20Object%20Reference) (OtherComp :type Primitive%20Component%20Object%20Reference) (OtherBodyIndex :type Integer))
  (bind _playerref (Variables|Default|GetPlayerRef))
  (bind _slidecamera (Variables|/Game/Blueprints/AmyPlayerCharacter/CharacterBlueprints/BP_PlayerCharacter.BP_PlayerCharacter_C|GetSlideCamera _playerref))
  (if (Components|Activation|IsActive _slidecamera)
    (Components|Activation|SetActive (Variables|/Game/Blueprints/AmyPlayerCharacter/CharacterBlueprints/BP_PlayerCharacter.BP_PlayerCharacter_C|GetFollowCamera (Variables|Default|GetPlayerRef)) true false)
    (Components|Activation|SetActive _slidecamera false false)))

(event EventBeginPlay)

(event Collision|EventActorBeginOverlap
  (params (OtherActor :type Actor%20Object%20Reference)))

(event EventTick
  (params (DeltaSeconds :type Float%20%28single-precision%29)))

(fn ConstructionScript)
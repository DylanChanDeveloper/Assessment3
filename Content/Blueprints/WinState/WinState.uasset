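; WinState is a goal trigger that ends the run when the player character overlaps its box collision.
; On BeginPlay it caches the player mesh's AmyAnim_BP instance.
; On overlap it sets that instance's GoalReached flag, which also guards against re-triggering, and starts a camera fade.
; After a delay matching the fade, it opens GameScene and clears the flag.
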(event OnComponentBeginOverlap(BoxCollision)
  (params (OverlappedComponent :type Primitive%20Component%20Object%20Reference) (OtherActor :type Actor%20Object%20Reference) (OtherComp :type Primitive%20Component%20Object%20Reference) (OtherBodyIndex :type Integer) (bFromSweep :type Boolean) (SweepResult :type Hit%20Result%20Structure%20%28by%20ref%29))
  ;[1 1 1] Comment
  (Utilities|Casting|CastToBP_PlayerCharacter OtherActor)
  (if (not (Variables|/Game/Character/Amy/Animations/AmyAnim_BP.AmyAnim_BP_C|GetGoalReached? (Variables|Default|GetAnimeRef)))
    (Variables|/Game/Character/Amy/Animations/AmyAnim_BP.AmyAnim_BP_C|SetGoalReached? (Variables|Default|GetAnimeRef) true)
    (CameraFades|StartCameraFade :self (Game|GetPlayerCameraManager 0) :ToAlpha 1.0 :Duration 4.0)
    (Utilities|FlowControl|Delay 4.0)
    (Game|OpenLevel(byName) "GameScene")
    (Variables|/Game/Character/Amy/Animations/AmyAnim_BP.AmyAnim_BP_C|SetGoalReached? (Variables|Default|GetAnimeRef) false)))

(event EventBeginPlay
  ;[1 1 1] Getting a reference to the animation blueprint so we can call the Goal reached boolean so we can call it below.
  (bind _asamy_anim_bp (Utilities|Casting|CastToAmyAnim_BP (Components|SkeletalMesh|GetAnimInstance (Variables|/Script/Engine.Character|GetMesh (Game|GetPlayerCharacter 0)))))
  (Variables|Default|SetAnimeRef _asamy_anim_bp))

(fn ConstructionScript)
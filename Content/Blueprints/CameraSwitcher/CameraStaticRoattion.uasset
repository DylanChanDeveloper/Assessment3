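; A trigger actor that switches the view to a fixed-position camera which turns to follow the player inside its box.
; Overlap by BP_PlayerCharacter blends the view to the ActiveCamera reference and starts RotateCamera.
; RotateCamera aims the camera at the cached player with a look-at rotation, re-calling itself after a short Delay instead of using Tick.
; Leaving the box returns the view to the player and clears CanRotate, ending the loop.
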(event OnComponentBeginOverlap(Box)
  (params (OverlappedComponent :type Primitive%20Component%20Object%20Reference) (OtherActor :type Actor%20Object%20Reference) (OtherComp :type Primitive%20Component%20Object%20Reference) (OtherBodyIndex :type Integer) (bFromSweep :type Boolean) (SweepResult :type Hit%20Result%20Structure%20%28by%20ref%29))
  ;[1 1 1] When entering the box overlap will cast to the player blueprint, then caches the player refernce(Just in case for future functionality). Next where setting up a camera transition by creating a variable called active camera and exposinging it so when can set the camera reference in the viewport.  we use set view target with blend to transition to the active camera. we then created a bool called canRotate and set its default value to false and call the rotate camera custom event node
  (bind _asbp_player_character (Utilities|Casting|CastToBP_PlayerCharacter OtherActor))
  (Variables|Default|SetPlayerCharacterRef _asbp_player_character)
  (Game|Player|SetViewTargetwithBlend (Game|GetPlayerController 0) (Variables|Default|GetActiveCamera) 1.0 "VTBlend_Linear" 0.0 false)
  (Variables|Default|SetCanRotate? true)
  (CallFunction|RotateCamera))

(event OnComponentEndOverlap(Box)
  (params (OverlappedComponent :type Primitive%20Component%20Object%20Reference) (OtherActor :type Actor%20Object%20Reference) (OtherComp :type Primitive%20Component%20Object%20Reference) (OtherBodyIndex :type Integer))
  ;[1 1 1] On exit sets the camera back to the players camera component set can roate to false
  (bind _asbp_player_character (Utilities|Casting|CastToBP_PlayerCharacter OtherActor))
  (Game|Player|SetViewTargetwithBlend (Game|GetPlayerController 0) _asbp_player_character 0.0 "VTBlend_Linear" 0.0 false)
  (Variables|Default|SetCanRotate? false))

(event Custom|Rotate%20Camera
  ;[1 1 1] If can rotate is true gets the active cameras location and the player character reference, then the return values are used in the find look at rotation which finds the rotation of the start location and the return value is used to set the actor rotation in this case the camera actor, then delays by 0.005 seconds to allow the code to run and calls the rotate camera function
  (if (Variables|Default|GetCanRotate?)
    (Transformation|SetActorRotation (Variables|Default|GetActiveCamera) (Math|Rotator|FindLookatRotation (Transformation|GetActorLocation (Variables|Default|GetActiveCamera)) (Transformation|GetActorLocation (Variables|Default|GetPlayerCharacterRef))))
    (Utilities|FlowControl|Delay 0.005)
    (CallFunction|RotateCamera)))

(event EventBeginPlay)

(event Collision|EventActorBeginOverlap
  (params (OtherActor :type Actor%20Object%20Reference)))

(event EventTick
  (params (DeltaSeconds :type Float%20%28single-precision%29)))

(fn ConstructionScript)
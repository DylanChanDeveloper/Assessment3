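; BP_CameraManager is a trigger volume that zooms the player camera out while BP_PlayerCharacter is inside it.
; Box overlap begin caches the player and sets CameraShift; any end overlap clears it.
; Tick eases the spring arm length toward a wide or default value with FInterpTo, whose speed is also scaled by delta time.
; The player reference is never cleared, and NewFunction is an uncalled duplicate of the zoom-in function.
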(event OnComponentBeginOverlap(BoxCollider)
  (params (OverlappedComponent :type Primitive%20Component%20Object%20Reference) (OtherActor :type Actor%20Object%20Reference) (OtherComp :type Primitive%20Component%20Object%20Reference) (OtherBodyIndex :type Integer) (bFromSweep :type Boolean) (SweepResult :type Hit%20Result%20Structure%20%28by%20ref%29))
  ;[1 1 1] Checks each frame if the camerashift is true if it is then checks if the player is valid, then finally adjusts the spring arm length. when the player exits the overlap sets the spring arm length back to normal
  (bind _asbp_player_character (Utilities|Casting|CastToBP_PlayerCharacter OtherActor))
  (Variables|Default|SetPlayer _asbp_player_character)
  (Variables|Default|SetCameraShift true))

(event OnComponentEndOverlap(BoxCollider)
  (params (OverlappedComponent :type Primitive%20Component%20Object%20Reference) (OtherActor :type Actor%20Object%20Reference) (OtherComp :type Primitive%20Component%20Object%20Reference) (OtherBodyIndex :type Integer))
  ;[1 1 1] when the player leaves camera shift is set to false.
  (Variables|Default|SetCameraShift false))

(event EventBeginPlay)

(event Collision|EventActorBeginOverlap
  (params (OtherActor :type Actor%20Object%20Reference)))

(event EventTick
  (params (DeltaSeconds :type Float%20%28single-precision%29))
  (bind _player (Variables|Default|GetPlayer))
  (bind _player_2 (Variables|Default|GetPlayer))
  (bind _springarm (Variables|/Game/Blueprints/AmyPlayerCharacter/CharacterBlueprints/BP_PlayerCharacter.BP_PlayerCharacter_C|GetSpringArm _player_2))
  (bind _springarm_2 (Variables|/Game/Blueprints/AmyPlayerCharacter/CharacterBlueprints/BP_PlayerCharacter.BP_PlayerCharacter_C|GetSpringArm _player))
  ;[1 1 1] Checks each frame if the camerashift is true if it is then checks if the player is valid, then finally adjusts the spring arm length. when the player exits the overlap sets the spring arm length back to normal
  (if (Variables|Default|GetCameraShift)
    (Utilities|IsValid _player_2
      (:Is%20Valid
        (CallFunction|ChangeSpringArmLength _springarm _springarm)))
    (else
      (Utilities|IsValid _player
        (:Is%20Valid
          (CallFunction|ChangeSpringArmLengthtoNormal _springarm_2 _springarm_2))))))

(fn ConstructionScript)

(fn ChangeSpringArmLength
  (params (FirstSpringArmTarget :type Spring%20Arm%20Component%20Object%20Reference) (SecondSpringArmTarget :type Spring%20Arm%20Component%20Object%20Reference))
  (bind _returnvalue (Utilities|Time|GetWorldDeltaSeconds))
  ;[1 1 1] Camera zoom out function interpolates the camera length out by 800 unreal units
  (Variables|/Script/Engine.SpringArmComponent|SetTargetArmLength FirstSpringArmTarget (Math|Interpolation|FInterpTo (Variables|/Script/Engine.SpringArmComponent|GetTargetArmLength SecondSpringArmTarget) 8e+02 _returnvalue (* _returnvalue 5e+01))))

(fn NewFunction
  (params (self2 :type Spring%20Arm%20Component%20Object%20Reference) (self3 :type Spring%20Arm%20Component%20Object%20Reference))
  (bind _returnvalue (Utilities|Time|GetWorldDeltaSeconds))
  (Variables|/Script/Engine.SpringArmComponent|SetTargetArmLength self2 (Math|Interpolation|FInterpTo (Variables|/Script/Engine.SpringArmComponent|GetTargetArmLength self3) 4e+02 _returnvalue (* _returnvalue 5e+01))))

(fn ChangeSpringArmLengthtoNormal
  (params (FirstSpringArmTarget :type Spring%20Arm%20Component%20Object%20Reference) (SecondSpringArmTarget :type Spring%20Arm%20Component%20Object%20Reference))
  (bind _returnvalue (Utilities|Time|GetWorldDeltaSeconds))
  ;[1 1 1] Camera zoom in function interpolates the camera length back to camera default value of 400 unreal units
  (Variables|/Script/Engine.SpringArmComponent|SetTargetArmLength FirstSpringArmTarget (Math|Interpolation|FInterpTo (Variables|/Script/Engine.SpringArmComponent|GetTargetArmLength SecondSpringArmTarget) 4e+02 _returnvalue (* _returnvalue 5e+01))))
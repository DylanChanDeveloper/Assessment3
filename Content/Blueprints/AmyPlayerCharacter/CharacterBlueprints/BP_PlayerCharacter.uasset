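; Player character Blueprint with Enhanced Input movement, jump cooldown, crouch, sprint and automatic slope sliding.
; BeginPlay fades the camera in, adds input mapping, caches the anim Blueprint and creates the UI.
; Tick interpolates the spring arm toward the player and checks floor angle, with separate enter and exit thresholds toggling walkable angle, rotation and slide animation.
; V swaps first- and third-person cameras, Q quits; spline camera test code is unused.
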(event Custom|CanSlide?
  (bind _charactermovement (Variables|Character|GetCharacterMovement))
  (bind _currentfloor (Variables|/Script/Engine.CharacterMovementComponent|GetCurrentFloor _charactermovement))
  (bind _hitresult (Utilities|Struct|BreakFindFloorResult _currentfloor))
  (bind _impactnormal (Collision|BreakHitResult _hitresult))
  ;[1 1 1] logic for custon third person camera as well as sliding logic
  (if (not (AI|Components|NavMovement|IsFalling (Variables|Character|GetCharacterMovement)))
    ;;[0.3515 0 0.4072] conditional statments for if the slope is greater than 30 and less than 10
    (bind _output_get (Variables|Default|SetslopeAngle (Class|KismetMathLibrary|DegAcos (Math|Vector|DotProduct _impactnormal "0.000000,0.000000,1.000000"))))
    (if (> _output_get 3e+01)
      ;;[0.3515 0 0.4072] Does this sequence once and when the sliding branch is false will run that code instead and reset the logic. Delay is 0.2 to allow a brief pause before the is sliding function runs
      (Utilities|FlowControl|DoOnce false :!label _label
        (:Completed
          (Utilities|FlowControl|Delay 0.2)
          ;;[0.09306 0 0.107] Collapsed function for is sliding logic
          (CallFunction|IsSliding (Math|Rotator|MakeRotfromZX _impactnormal (Transformation|GetActorForwardVector)))))
      (else
        ;;[0.3515 0 0.4072] Conditional statments for not sliding function
        (if (< _output_get 1e+01)
          (if (Variables|/Game/Character/Amy/Animations/AmyAnim_BP.AmyAnim_BP_C|GetIsSliding? (Variables|Default|GetAnimBPRef))
            ;;[0.3372 0.009721 0.3813] collapsed functions for is not sliding logic
            (CallFunction|NotSliding)
            (goto _label Reset)))))))

(event Input|EnhancedActionEvents|EnhancedInputActionIA_Jump
  (params (ActionValue :type Boolean) (ElapsedSeconds :type Float%20%28double-precision%29) (TriggeredSeconds :type Float%20%28double-precision%29) (InputAction :type Input%20Action%20Object%20Reference :default "/Game/Blueprints/AmyPlayerCharacter/Input/IA_Jump.IA_Jump"))
  ;[0.187 1 0.0904] Jump, using can jump bool to stop the player from spamming jump and allow the animation to run its course.
  (:Triggered
    (if (Variables|Default|GetCan%20Jump?)
      (Character|Jump)
      (Variables|Default|SetCan%20Jump? false)
      (Utilities|FlowControl|Delay 1.0)
      (Variables|Default|SetCan%20Jump? true)))
  (:Completed
    (Character|StopJumping)))

(event Input|EnhancedActionEvents|EnhancedInputActionIA_Look
  (params (ActionValue :type Vector%202D%20Structure) (ElapsedSeconds :type Float%20%28double-precision%29) (TriggeredSeconds :type Float%20%28double-precision%29) (InputAction :type Input%20Action%20Object%20Reference :default "/Game/Blueprints/AmyPlayerCharacter/Input/IA_Look.IA_Look"))
  ;[0.04388 0.8803 1] CameraInput
  (:Triggered
    ;;[1 1 1] Look Left/Right
    (Pawn|Input|AddControllerYawInput (.x ActionValue))
    ;;[1 1 1] Look Up/Down
    (Pawn|Input|AddControllerPitchInput (.y ActionValue))))

(event Input|EnhancedActionEvents|EnhancedInputActionIA_Movement
  (params (ActionValue :type Vector%202D%20Structure) (ElapsedSeconds :type Float%20%28double-precision%29) (TriggeredSeconds :type Float%20%28double-precision%29) (InputAction :type Input%20Action%20Object%20Reference :default "/Game/Blueprints/AmyPlayerCharacter/Input/IA_Movement.IA_Movement"))
  (bind _returnvalue (Pawn|GetControlRotation :!class /Script/Engine.Pawn))
  ;[1 0.9886 0.1872] MovementInput: flipped values and multiplied the y value so the character can move in the appropriate direction
  (:Triggered
    (Pawn|Input|AddMovementInput (Math|Vector|GetRightVector (Math|Rotator|MakeRotator (.roll _returnvalue) 0.0 (.yaw _returnvalue))) (* (.y ActionValue) -1.0) false)
    (Pawn|Input|AddMovementInput (Math|Vector|GetForwardVector (Math|Rotator|MakeRotator 0.0 0.0 (.yaw (Pawn|GetControlRotation :!class /Script/Engine.Pawn)))) (.x ActionValue) false)))

(event Input|EnhancedActionEvents|EnhancedInputActionIK_Crouch
  (params (ActionValue :type Boolean) (ElapsedSeconds :type Float%20%28double-precision%29) (TriggeredSeconds :type Float%20%28double-precision%29) (InputAction :type Input%20Action%20Object%20Reference :default "/Game/Blueprints/AmyPlayerCharacter/Input/IK_Crouch.IK_Crouch"))
  ;[1 1 1] Crounch: using unreals new input functions crouch and uncrouch. Note in the character movement, can crouch bool must be ticked.
  (:Started
    (Character|Crouch))
  (:Completed
    (Character|UnCrouch)))

(event Input|EnhancedActionEvents|EnhancedInputActionIK_Sprint
  (params (ActionValue :type Vector%202D%20Structure) (ElapsedSeconds :type Float%20%28double-precision%29) (TriggeredSeconds :type Float%20%28double-precision%29) (InputAction :type Input%20Action%20Object%20Reference :default "/Game/Blueprints/AmyPlayerCharacter/Input/IK_Sprint.IK_Sprint"))
  ;[1 0.1349 0.1647] Sprint logic get velcoity if vector a velocity is not the same as vector B's velocity them the start sprint function will run. e.g. movement speed at 600. Completed executes when the player lets go of the sprint input and sets the character movement value back to its orginal speed
  (:Triggered
    (if (Utilities|Operators|NotEqual(!=) :A (Transformation|GetVelocity))
      (CallFunction|StartSprint)))
  (:Completed
    (CallFunction|StopSprint)))

(event EventBeginPlay
  ;[1 1 1] Adds input mapping, altered at the start so theres a camera fade. As well as getting references ti the anime blueprint to access animation variables to use to change the animations. Finally creating and adding the widget blueprint to the viewport
  (Utilities|FlowControl|Sequence
    (:then_0
      (CameraFades|StartCameraFade :self (Game|GetPlayerCameraManager 0) :FromAlpha 1.0 :Duration 3.0)
      (Utilities|FlowControl|Sequence
        (:then_0
          (bind _asplayer_controller (Utilities|Casting|CastToPlayerController (Pawn|GetController)))
          (Utilities|IsValid (PlayerController|LocalPlayerSubsystems|GetEnhancedInputLocalPlayerSubsystem _asplayer_controller)
            (:Is%20Valid
              (Input|AddMappingContext (PlayerController|LocalPlayerSubsystems|GetEnhancedInputLocalPlayerSubsystem _asplayer_controller) "/Game/Blueprints/AmyPlayerCharacter/Input/IMC_Character.IMC_Character" 0 "(bIgnoreAllPressedKeysUntilRelease=True,bForceImmediately=False)"))))))
    (:then_1
      (bind _asamy_anim_bp (Utilities|Casting|CastToAmyAnim_BP (Components|SkeletalMesh|GetAnimInstance (Variables|Character|GetMesh))))
      (Variables|Default|SetAnimBPRef _asamy_anim_bp))
    (:then_2
      (bind _returnvalue (UserInterface|CreateWidget "/Game/UI/PlayerUI.PlayerUI_C"))
      (UserInterface|Viewport|AddtoViewport _returnvalue 0))))

(event EventTick
  (params (DeltaSeconds :type Float%20%28single-precision%29))
  (bind _springarm (Variables|Default|GetSpringArm))
  ;[1 1 1] logic for custon third person camera as well as sliding logic
  (Utilities|FlowControl|Sequence
    (:then_0
      (Transformation|SetWorldLocation _springarm (Math|Interpolation|VInterpTo (Transformation|GetWorldLocation _springarm) (Transformation|GetActorLocation) (Utilities|Time|GetWorldDeltaSeconds) 1.8) false false))
    (:then_1
      ;;[0.8569 0 1] Constantly checking the can slid custom function with event tick
      (CallFunction|CanSlide?))))

(event Input|KeyboardEvents|V
  (params (Key :type Key%20Structure :default "None"))
  (bind _followcamera (Variables|Default|GetFollowCamera))
  (bind _firstpersoncamera (Variables|Default|GetFirstPersonCamera))
  ;[1 0.4 0.2294] CameraToggle between first and third person. When V is pressed checks if the Follow camera (Third person camera) is active if this is true sets the first person camera active and sets the follow camera un active for the true statment. Oppsite for the false staement
  (:Pressed
    (if (Components|Activation|IsActive (Variables|Default|GetFollowCamera))
      (Components|Activation|SetActive _firstpersoncamera true false)
      (Components|Activation|SetActive _followcamera false false)
      (Variables|Default|SetbUseControllerRotationYaw true)
      (else
        (Components|Activation|SetActive _firstpersoncamera false false)
        (Components|Activation|SetActive _followcamera true false)
        (Variables|Default|SetbUseControllerRotationYaw false)))))

(event Input|KeyboardEvents|Q
  (params (Key :type Key%20Structure :default "None"))
  ;[1 1 1] Quit
  (:Pressed
    (Game|QuitGame 0 "Quit" false)))

(fn ConstructionScript)

(fn StartSprint
  ;[1 1 1] Sets character speed to 600
  (Variables|/Script/Engine.CharacterMovementComponent|SetMaxWalkSpeed (Variables|Character|GetCharacterMovement) 6e+02))

(fn StopSprint
  ;[1 1 1] Sets character speed to 200 orginal walking speed
  (Variables|/Script/Engine.CharacterMovementComponent|SetMaxWalkSpeed (Variables|Character|GetCharacterMovement) 2e+02))

(fn NotSliding
  ;[1 1 1] Set the walkable floor back to default values and the actor rotation back to normal., disables the is sliding bool for sliding animation so the player is back to its orginal walking state
  (Pawn|Components|CharacterMovement|SetWalkableFloorAngle (Variables|Character|GetCharacterMovement) 44.765083)
  (Variables|/Game/Character/Amy/Animations/AmyAnim_BP.AmyAnim_BP_C|SetIsSliding? (Variables|Default|GetAnimBPRef) false)
  (Transformation|SetActorRotation (Math|Rotator|MakeRotator 0.0 0.0 (.yaw (Transformation|GetActorRotation))))
  (Variables|/Script/Engine.CharacterMovementComponent|SetbOrientRotationToMovement (Variables|Character|GetCharacterMovement) true))

(fn IsSliding
  (params (NewRotation :type Rotator))
  ;[1 1 1] Set the walkable floor angle as well as setting the player rotation to be the slope angle, enables the is sliding bool for sliding animation to play and turning of the roatation movement so the player cant move rotation during animation
  (Pawn|Components|CharacterMovement|SetWalkableFloorAngle (Variables|Character|GetCharacterMovement) 1.0)
  (Transformation|SetActorRotation NewRotation)
  (Variables|/Game/Character/Amy/Animations/AmyAnim_BP.AmyAnim_BP_C|SetIsSliding? (Variables|Default|GetAnimBPRef) true)
  (Variables|/Script/Engine.CharacterMovementComponent|SetbOrientRotationToMovement (Variables|Character|GetCharacterMovement) false))
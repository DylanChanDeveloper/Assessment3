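; MovableCube is a cube that the player character can push.
; Two overlap volumes, one for the X axis and one for the Y axis, enable physics simulation on the cube when BP_PlayerCharacter enters and disable it on exit.
; The same events toggle the character's IsPushing flag, which the comments say drives the pushing animation.
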(event OnComponentBeginOverlap(yaxiscollsion)
  (params (OverlappedComponent :type Primitive%20Component%20Object%20Reference) (OtherActor :type Actor%20Object%20Reference) (OtherComp :type Primitive%20Component%20Object%20Reference) (OtherBodyIndex :type Integer) (bFromSweep :type Boolean) (SweepResult :type Hit%20Result%20Structure%20%28by%20ref%29))
  ;[1 1 1] Y Axis collision, when the player enters the overlap sets the box physics to true and the is pushing animegraph bool varible to true to play the pushing animation, when the player leaves the box collision turns off the physics and animation
  (bind _asbp_player_character (Utilities|Casting|CastToBP_PlayerCharacter OtherActor))
  (Physics|SetSimulatePhysics (Variables|Default|GetCube) true)
  (Variables|/Game/Blueprints/AmyPlayerCharacter/CharacterBlueprints/BP_PlayerCharacter.BP_PlayerCharacter_C|SetIsPushing? _asbp_player_character true))

(event OnComponentEndOverlap(yaxiscollsion)
  (params (OverlappedComponent :type Primitive%20Component%20Object%20Reference) (OtherActor :type Actor%20Object%20Reference) (OtherComp :type Primitive%20Component%20Object%20Reference) (OtherBodyIndex :type Integer))
  ;[1 1 1] Y Axis collision, when the player enters the overlap sets the box physics to true and the is pushing animegraph bool varible to true to play the pushing animation, when the player leaves the box collision turns off the physics and animation
  (bind _asbp_player_character (Utilities|Casting|CastToBP_PlayerCharacter OtherActor))
  (Physics|SetSimulatePhysics (Variables|Default|GetCube) false)
  (Variables|/Game/Blueprints/AmyPlayerCharacter/CharacterBlueprints/BP_PlayerCharacter.BP_PlayerCharacter_C|SetIsPushing? _asbp_player_character false))

(event OnComponentBeginOverlap(xaxiscollsion)
  (params (OverlappedComponent :type Primitive%20Component%20Object%20Reference) (OtherActor :type Actor%20Object%20Reference) (OtherComp :type Primitive%20Component%20Object%20Reference) (OtherBodyIndex :type Integer) (bFromSweep :type Boolean) (SweepResult :type Hit%20Result%20Structure%20%28by%20ref%29))
  ;[1 1 1] X Axis collision, same logic as y axiss exect for the x axis
  (bind _asbp_player_character (Utilities|Casting|CastToBP_PlayerCharacter OtherActor))
  (Physics|SetSimulatePhysics (Variables|Default|GetCube) true)
  (Variables|/Game/Blueprints/AmyPlayerCharacter/CharacterBlueprints/BP_PlayerCharacter.BP_PlayerCharacter_C|SetIsPushing? _asbp_player_character true))

(event OnComponentEndOverlap(xaxiscollsion)
  (params (OverlappedComponent :type Primitive%20Component%20Object%20Reference) (OtherActor :type Actor%20Object%20Reference) (OtherComp :type Primitive%20Component%20Object%20Reference) (OtherBodyIndex :type Integer))
  ;[1 1 1] X Axis collision, same logic as y axiss exect for the x axis
  (bind _asbp_player_character (Utilities|Casting|CastToBP_PlayerCharacter OtherActor))
  (Physics|SetSimulatePhysics (Variables|Default|GetCube) false)
  (Variables|/Game/Blueprints/AmyPlayerCharacter/CharacterBlueprints/BP_PlayerCharacter.BP_PlayerCharacter_C|SetIsPushing? _asbp_player_character false))

(fn ConstructionScript)